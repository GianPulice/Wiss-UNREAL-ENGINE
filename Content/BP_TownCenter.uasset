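; BP_TownCenter is a town-center actor that switches Wwise town ambience on and off by player proximity.
; It caches the third-person player character on BeginPlay and reads that character's DistanceToTown value every Tick.
; A playing flag makes it post the Ak event once inside a fixed radius and issue a Stop action with a transition once outside.
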(event `self.ReceiveBeginPlay`
  (bind _asbp_third_person_character (cast `/Game/ThirdPerson/Blueprints/BP_ThirdPersonCharacter` (`GameplayStatics.GetPlayerCharacter` 0)))
  (set `self.playerRef` _asbp_third_person_character))

(event `self.ReceiveTick`
  (params (DeltaSeconds :type "Float (single-precision)"))
  (bind _ak_event_town (`self.Ak Event Town`))
  (bind _output_get (set `self.DistanceFromPlayer` (`/Game/ThirdPerson/Blueprints/BP_ThirdPersonCharacter.DistanceToTown` (`self.playerRef`))))
  (if (< _output_get 75.0)
    (if (not (`self.bTownAmbiencePlaying`))
      (`AkGameplayStatics.PostEvent` _ak_event_town)
      (set `self.bTownAmbiencePlaying` true))
    (elif (`self.bTownAmbiencePlaying`)
      (`AkAudioEvent.ExecuteAction` _ak_event_town "Stop" null (`self.PlayingID`) 5 "Linear")
      (set `self.bTownAmbiencePlaying` false))))

(fn `UserConstructionScript`)